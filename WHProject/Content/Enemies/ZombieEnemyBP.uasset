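; ZombieEnemyBP is an enemy Blueprint that acts on its Target when it gets close during a specific phase.
; On Tick, while Phase is 4 and the Target is within a short distance, it teleports the Target to the world origin and advances Phase to 5.
; The move is an unswept SetActorLocation; the Range variable is unused, with the distance threshold hardcoded, and the construction script is empty.
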(event EventTick
  (params (DeltaSeconds :type Float%20%28single-precision%29))
  (if (and (== (Variables|Default|GetPhase) 4) (<= (Math|Vector|Distance(Vector) (Transformation|GetActorLocation (Variables|Default|GetTarget)) (Transformation|GetActorLocation)) 1e+02))
    (Transformation|SetActorLocation (Variables|Default|GetTarget) "0, 0, 0" false false)
    (Variables|Default|SetPhase 5)))

(fn ConstructionScript)